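; Main game mode that tracks the player, enemies, checkpoints, game over and pause menu.
; A one-second timer finds which NavMeshBoundsVolume the grounded player is on and broadcasts changes to notify AI.
; Registered enemies get their current volume and feed spawn and kill counters that print a victory message once spawners are gone.
; Respawn returns the player to the last checkpoint with life damage, while game over reloads the level.
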(event Custom|UpdateCheckPoint
  (params (CheckPointOverlapped :type BP%20Check%20Point%20Object%20Reference))
  (Variables|Default|SetLastCheckPointOverlapped CheckPointOverlapped))

(event Custom|RespawnPlayer
  (bind _lastcheckpointoverlapped (Variables|Default|GetLastCheckPointOverlapped))
  (bind _returnvalue (Default|GetCheckPointRespawnTransform _lastcheckpointoverlapped))
  ;[1 1 1] RespawnPlayer
  (Utilities|IsValid _lastcheckpointoverlapped
    (:Is%20Valid
      (Transformation|SetActorLocation (Game|Player|GetPlayerPawn 0) (.location _returnvalue) false false)
      (Pawn|SetControlRotation (Game|GetPlayerController 0) (.rotation _returnvalue))
      (Default|UpdateLife (Variables|Default|GetPlayer) (Variables|CanBeModified|GetLifeDamageAfterRespawn)))))

(event Custom|GameOver
  ;[1 0.03018 0] Game Over
  (Development|PrintString "Game Over...  Reloading Game in 2 seconds" true true "(R=1.000000,G=0.000000,B=0.000000,A=1.000000)")
  (Utilities|FlowControl|Delay 2.0)
  (bind _returnvalue (Game|GetCurrentLevelName true))
  (Game|OpenLevel(byName) (Utilities|String|StringToName _returnvalue)))

(event Custom|RegisterEnemy
  (params (NewEnemy :type BP%20Base%20Enemy%20Object%20Reference))
  ;[0 0.5845 1] Register / Unregister Enemies          Called when a new enemy is spawned or when he has been killed
  (Utilities|Array|AddUnique (Variables|Default|GetEnemies) NewEnemy)
  (Math|Integer|IncrementInt (Variables|Default|GetEnemiesSpawned)
    (:%20%20
      (bind _array_element (Utilities|Array|ForEachLoopwithBreak (Variables|Default|GetNavMeshVolumes) :!label _label)
        (:LoopBody
          (bind _result (CallFunction|IsCharacteronNavMesh NewEnemy _array_element))
          (if _result
            (Variables|/Game/Blueprints/Enemies/BP_BaseEnemy.BP_BaseEnemy_C|SetcurrentNavMesh NewEnemy _array_element)
            (goto _label Break)))))))

(event Custom|RegisterPlayer
  ;[1 1 1] Save the player reference
  (bind _returnvalue (Actor|GetActorOfClass "/Game/FirstPersonBP/Blueprints/FirstPersonCharacter.FirstPersonCharacter_C"))
  (Variables|Default|SetPlayer _returnvalue))

(event Custom|UnregisterEnemy
  (params (KilledEnemy :type BP%20Base%20Enemy%20Object%20Reference))
  ;[0 0.5845 1] Register / Unregister Enemies          Called when a new enemy is spawned or when he has been killed
  (bind _returnvalue (Utilities|Array|RemoveItem (Variables|Default|GetEnemies) KilledEnemy))
  (if _returnvalue
    (Math|Integer|IncrementInt (Variables|Default|GetEnemiesKilled)
      (:%20%20
        (bind _outactors (Actor|GetAllActorsOfClass "/Game/Blueprints/BP_EnemySpawner.BP_EnemySpawner_C")) ; Not perfect, just for the test
        (if (and (== (Utilities|Array|Length _outactors) 0) (== (Variables|Default|GetEnemiesKilled) (Variables|Default|GetEnemiesSpawned)))
          (Development|PrintString "You killed all the enemies !" true true "(R=1.000000,G=0.145191,B=0.000000,A=1.000000)"))))
    (else
      (Development|PrintString "Try to remove an enemy who hasn't been registered..." true true "(R=1.000000,G=0.000000,B=0.000000,A=1.000000)" 3.0))))

(event Custom|CheckPlayerOnNavMesh
  (bind _player (Variables|Default|GetPlayer))
  ;[1 1 1] Called each 1 second to check if the player is on a new NavMeshVolume. If YES, IA are notified.
  (Utilities|IsValid _player
    (:Is%20Valid
      (if (AI|Components|NavMovement|IsMovingonGround (Variables|/Script/Engine.Character|GetCharacterMovement _player))
        (bind _result (CallFunction|IsCharacteronNavMesh (Variables|Default|GetPlayer) (Variables|/Game/FirstPersonBP/Blueprints/FirstPersonCharacter.FirstPersonCharacter_C|GetCurrentNavMesh _player)))
        (if (not _result)
          (CallFunction|CheckonAllNavMeshVolumes))))))

(event Custom|PauseMenu
  (bind _returnvalue (Game|GetPlayerController 0))
  ;[1 1 1] Game Pause Menu
  (Utilities|FlowControl|FlipFlop
    (:A
      (bind _returnvalue_2 (UserInterface|CreateWidget "/Game/Blueprints/Widgets/WGP_PauseMenu.WGP_PauseMenu_C"))
      (UserInterface|Viewport|AddtoViewport _returnvalue_2 0)
      (Game|SetGamePaused true)
      (Variables|/Script/Engine.PlayerController|SetbShowMouseCursor _returnvalue true))
    (:B
      (Widget|RemovefromParent _returnvalue_2)
      (Game|SetGamePaused false)
      (Variables|/Script/Engine.PlayerController|SetbShowMouseCursor _returnvalue false))))

(event EventBeginPlay
  ;[1 1 1] Init data
  (CallFunction|RegisterPlayer)
  (bind _outactors (Actor|GetAllActorsOfClass "/Script/NavigationSystem.NavMeshBoundsVolume"))
  (Variables|Default|SetNavMeshVolumes _outactors)
  (Utilities|Time|SetTimerbyEvent (delegate Custom|CheckPlayerOnNavMesh) 1.0 true))

(fn ConstructionScript)

(fn CheckonAllNavMeshVolumes
  (bind _array_element (Utilities|Array|ForEachLoopwithBreak (Variables|Default|GetNavMeshVolumes) :!label _label)
    (:LoopBody
      (bind _result (CallFunction|IsCharacteronNavMesh (Variables|Default|GetPlayer) _array_element))
      (bind _output_get (LocalVariables|SetIsOverlappingOne _result))
      (if _output_get
        (Variables|/Game/FirstPersonBP/Blueprints/FirstPersonCharacter.FirstPersonCharacter_C|SetCurrentNavMesh (Variables|Default|GetPlayer) _array_element)
        (Default|CallOnPlayerIsOverlappingNewNavMesh)
        (goto _label Break)))
    (:Completed
      ;[1 1 1] If the player is not above a navMeshVolume, currentNavMesh = null
      (if (not (LocalVariables|GetIsOverlappingOne))
        (Variables|/Game/FirstPersonBP/Blueprints/FirstPersonCharacter.FirstPersonCharacter_C|SetCurrentNavMesh (Variables|Default|GetPlayer) 0)
        (Default|CallOnPlayerIsOverlappingNewNavMesh)))))