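; Laser gun weapon that shows a Niagara beam while firing and damages actors tagged Enemy.
; StartFire and StopFire toggle the beam and actor Tick, which is off by default.
; Tick line-traces along the Arrow, ending the beam at the impact point only for enemy hits.
; A Delay in a custom event throttles per-frame damage calls to about fifteen hits per second.
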(event Custom|ApplyDamageEachNSeconds
  (params (DamagedActor :type Actor%20Object%20Reference))
  ;[1 1 1] Linecast then damage if it's an enemy
  ;;[0.3531 0.9652 1] 1/15 => 15 hits chaque seconde
  (Utilities|FlowControl|Delay 0.066667)
  (Game|Damage|ApplyDamage DamagedActor (Variables|Default|GetDamage) 0 0))

(event EventBeginPlay
  (Actor|Tick|SetActorTickEnabled false))

(event EventStartFire
  (bind _niagara (Variables|Default|GetNiagara))
  ;[1 1 1] Laser fx
  (Components|Activation|Activate _niagara true)
  (Effects|Components|ParticleSystem|SetColorParameter _niagara "User.Color" (Variables|Default|GetLaserColor))
  (Actor|Tick|SetActorTickEnabled true))

(event EventStopFire
  ;[1 1 1] Laser fx
  (Components|Activation|Deactivate (Variables|Default|GetNiagara))
  (Actor|Tick|SetActorTickEnabled false))

(event EventTick
  (params (DeltaSeconds :type Float%20%28single-precision%29))
  (bind _arrow (Variables|Default|GetArrow))
  (bind _laserlength (Variables|Default|GetLaserLength))
  (bind _returnvalue (Math|Vector|GetForwardVector _arrow))
  (bind _returnvalue_2 (Transformation|GetWorldLocation _arrow))
  (bind _returnvalue_3 (* _returnvalue _laserlength))
  (bind _returnvalue_4 (+ _returnvalue_2 _returnvalue_3))
  ;[1 1 1] Linecast then damage if it's an enemy
  (Effects|Components|ParticleSystem|SetVectorParameter (Variables|Default|GetNiagara) "User.End" _returnvalue_4)
  (bind (_outhit _returnvalue_5) (Collision|LineTraceByChannel _returnvalue_2 _returnvalue_4 "TraceTypeQuery1" false 0 "None"))
  (if _returnvalue_5
    (if (Actor|ActorHasTag (.HitActor (Collision|BreakHitResult _outhit)) "Enemy")
      (Effects|Components|ParticleSystem|SetVectorParameter (Variables|Default|GetNiagara) "User.End" (.ImpactPoint (Collision|BreakHitResult _outhit)))
      (CallFunction|ApplyDamageEachNSeconds (.HitActor (Collision|BreakHitResult _outhit))))))

(fn ConstructionScript
  (|CallParentFunction))